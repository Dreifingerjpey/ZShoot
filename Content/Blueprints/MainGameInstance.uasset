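; The game instance that opens the game's menu screens: main menu, graphics settings, lobby, character creation, profile and map creator.
; Each event lazily creates and caches its widget, then typically adds it to the viewport with UI-only input and a visible cursor.
; Profile leaves the cursor setting untouched, its cursor node being unwired.
; The map event only creates its widget on first call, displaying it on later calls.
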(event `Show Main Menue`
  (bind _returnvalue (`GameplayStatics.GetPlayerController` 0))
  ;[1 1 1] Show Main Menue
  (`/Engine/EditorBlueprintResources/StandardMacros.IsValid` (`self.MainMenue`)
    (:`Is Valid`
      _)
    (:`Is Not Valid`
      (bind _returnvalue_2 (`|CreateWidget` "/Game/UI/Visuell/MainMenue/MainMenue.MainMenue_C" _returnvalue))
      (set `self.MainMenue` _returnvalue_2)))
  (`UserWidget.AddToViewport` (`self.MainMenue`) 0)
  (`WidgetBlueprintLibrary.SetInputMode_UIOnlyEx` _returnvalue)
  (set `PlayerController.bShowMouseCursor` true _returnvalue))

(event `Show Graphic Menue`
  (bind _returnvalue (`GameplayStatics.GetPlayerController` 0))
  ;[1 1 1] Graphic Menue
  (`/Engine/EditorBlueprintResources/StandardMacros.IsValid` (`self.GraphicSettings`)
    (:`Is Valid`
      _)
    (:`Is Not Valid`
      (bind _returnvalue_2 (`|CreateWidget` "/Game/UI/Visuell/MainMenue/GraphicSettings.GraphicSettings_C" _returnvalue))
      (set `self.GraphicSettings` _returnvalue_2)))
  (`UserWidget.AddToViewport` (`self.GraphicSettings`) 0)
  (`WidgetBlueprintLibrary.SetInputMode_UIOnlyEx` _returnvalue)
  (set `PlayerController.bShowMouseCursor` true _returnvalue))

(event `Show Lobby`
  (bind _returnvalue (`GameplayStatics.GetPlayerController` 0))
  ;[1 1 1] Lobby
  (`/Engine/EditorBlueprintResources/StandardMacros.IsValid` (`self.Lobby`)
    (:`Is Valid`
      _)
    (:`Is Not Valid`
      (bind _returnvalue_2 (`|CreateWidget` "/Game/UI/Visuell/MainMenue/Lobby.Lobby_C" _returnvalue))
      (set `self.Lobby` _returnvalue_2)))
  (`UserWidget.AddToViewport` (`self.Lobby`) 0)
  (`WidgetBlueprintLibrary.SetInputMode_UIOnlyEx` _returnvalue)
  (set `PlayerController.bShowMouseCursor` true _returnvalue))

(event `Show CharacterCreation`
  (bind _returnvalue (`GameplayStatics.GetPlayerController` 0))
  ;[1 1 1] Character Creation
  (`/Engine/EditorBlueprintResources/StandardMacros.IsValid` (`self.Character Creation`)
    (:`Is Valid`
      _)
    (:`Is Not Valid`
      (bind _returnvalue_2 (`|CreateWidget` "/Game/UI/Visuell/MainMenue/CharacterCreator.CharacterCreator_C" _returnvalue))
      (set `self.Character Creation` _returnvalue_2)))
  (`UserWidget.AddToViewport` (`self.Character Creation`) 0)
  (`WidgetBlueprintLibrary.SetInputMode_UIOnlyEx` _returnvalue)
  (set `PlayerController.bShowMouseCursor` true _returnvalue))

(event `show Profile`
  (bind _returnvalue (`GameplayStatics.GetPlayerController` 0))
  ;[1 1 1] Profile
  (`/Engine/EditorBlueprintResources/StandardMacros.IsValid` (`self.Profile`)
    (:`Is Valid`
      _)
    (:`Is Not Valid`
      (bind _returnvalue_2 (`|CreateWidget` "/Game/UI/Visuell/MainMenue/Profile.Profile_C" _returnvalue))
      (set `self.Profile` _returnvalue_2)))
  (`UserWidget.AddToViewport` (`self.Profile`) 0)
  (`WidgetBlueprintLibrary.SetInputMode_UIOnlyEx` _returnvalue))

(event `show Map Preview Menue`
  (bind _returnvalue (`GameplayStatics.GetPlayerController` 0))
  ;[1 1 1] Map  Menue
  (`/Engine/EditorBlueprintResources/StandardMacros.IsValid` (`self.MapCreator`)
    (:`Is Valid`
      (`UserWidget.AddToViewport` (`self.MapCreator`) 0)
      (`WidgetBlueprintLibrary.SetInputMode_UIOnlyEx` _returnvalue)
      (set `PlayerController.bShowMouseCursor` true _returnvalue))
    (:`Is Not Valid`
      (bind _returnvalue_2 (`|CreateWidget` "/Game/UI/Visuell/MainMenue/MapCreator.MapCreator_C" _returnvalue))
      (set `self.MapCreator` _returnvalue_2))))